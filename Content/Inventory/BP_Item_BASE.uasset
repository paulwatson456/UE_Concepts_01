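; Base item Blueprint, likely for inventory pickups, that animates its ItemVisualRep component with an idle bob and turn.
; BeginPlay stores the visual's relative location as the high point and derives a low point 20 units below.
; Bob eases the component between both points with a half-turn and back, pausing briefly, then calls itself to loop.
; FeedbackPickup is an empty event, and the construction script does nothing.
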(event `self.ReceiveBeginPlay`
  (set `self.HeightOfMovment` (`SceneComponent.RelativeLocation` (`self.ItemVisualRep`)))
  (set `self.LowOfMovment` (- (`self.HeightOfMovment`) (0.0 0.0 20.0)))
  (`self.Bob`))

(event `Bob`
  (`KismetSystemLibrary.MoveComponentTo` (`self.ItemVisualRep`) (`self.LowOfMovment`) (struct :`Yaw` 180.0) true true 0.7)
  (`KismetSystemLibrary.Delay` 0.2)
  (`KismetSystemLibrary.MoveComponentTo` (`self.ItemVisualRep`) (`self.HeightOfMovment`) (struct) true true 0.7)
  (`KismetSystemLibrary.Delay` 0.2)
  (`self.Bob`))

(event `FeedbackPickup`)

(fn `UserConstructionScript`)