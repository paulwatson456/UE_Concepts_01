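; Test actor that spawns collectable objects at random, non-repeating picks from six point components.
; On BeginPlay it enables input, refills the point array, then loops three times: shuffle, spawn BP_CollectableObject_Base at the first point, remove that point.
; The O key repeats this with a fresh array, while P prints a debug message and spawns from the remaining points without refilling.
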(event EventBeginPlay
  (Input|EnableInput (Game|GetPlayerController 0))
  (Variables|Default|SetSpawnPoints (Utilities|Array|MakeArray (Variables|Default|GetPoint%203) (Variables|Default|GetPoint%202) (Variables|Default|GetPoint%201) (Variables|Default|GetPoint%204) (Variables|Default|GetPoint%205) (Variables|Default|GetPoint%206)))
  (for _index (range 0 2)
    (Utilities|Array|Shuffle (Variables|Default|GetSpawnPoints))
    (Game|SpawnActorfromClass "/Game/PCG/BP_CollectableObject_Base.BP_CollectableObject_Base_C" (Math|Conversions|ToTransform(Vector) (Transformation|GetWorldLocation (Utilities|Array|Get(acopy) (Variables|Default|GetSpawnPoints)))) "Undefined" "MultiplyWithRoot" 0 0)
    (Utilities|Array|RemoveIndex (Variables|Default|GetSpawnPoints))))

(event Collision|EventActorBeginOverlap
  (params (OtherActor :type Actor%20Object%20Reference)))

(event EventTick
  (params (DeltaSeconds :type Float%20%28single-precision%29)))

(event Input|KeyboardEvents|P
  (params (Key :type Key%20Structure :default "None"))
  (:Pressed
    (Development|PrintString "Hello")
    (for _index (range 0 2)
      (Utilities|Array|Shuffle (Variables|Default|GetSpawnPoints))
      (Game|SpawnActorfromClass "/Game/PCG/BP_CollectableObject_Base.BP_CollectableObject_Base_C" (Math|Conversions|ToTransform(Vector) (Transformation|GetWorldLocation (Utilities|Array|Get(acopy) (Variables|Default|GetSpawnPoints)))) "Undefined" "MultiplyWithRoot" 0 0)
      (Utilities|Array|RemoveIndex (Variables|Default|GetSpawnPoints)))))

(event Input|KeyboardEvents|O
  (params (Key :type Key%20Structure :default "None"))
  (:Pressed
    (Variables|Default|SetSpawnPoints (Utilities|Array|MakeArray (Variables|Default|GetPoint%203) (Variables|Default|GetPoint%202) (Variables|Default|GetPoint%201) (Variables|Default|GetPoint%204) (Variables|Default|GetPoint%205) (Variables|Default|GetPoint%206)))
    (for _index (range 0 2)
      (Utilities|Array|Shuffle (Variables|Default|GetSpawnPoints))
      (Game|SpawnActorfromClass "/Game/PCG/BP_CollectableObject_Base.BP_CollectableObject_Base_C" (Math|Conversions|ToTransform(Vector) (Transformation|GetWorldLocation (Utilities|Array|Get(acopy) (Variables|Default|GetSpawnPoints)))) "Undefined" "MultiplyWithRoot" 0 0)
      (Utilities|Array|RemoveIndex (Variables|Default|GetSpawnPoints)))))

(fn ConstructionScript)