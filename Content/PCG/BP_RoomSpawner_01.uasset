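; BP_RoomSpawner_01 procedurally builds a linear chain of rooms when play begins.
; It spawns BP_StartRoom_A at its own location, then fifteen random picks from MiddleRooms, and closes with BP_EndRoom_A.
; Each room is placed at the EndPoint world location of the previous one, passing only position into the spawn transform.
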(event EventBeginPlay
  (bind _returnvalue (Game|SpawnActorfromClass "/Game/PCG/BP_StartRoom_A.BP_StartRoom_A_C" (Math|Conversions|ToTransform(Vector) (Transformation|GetWorldLocation (Variables|Default|GetDefaultSceneRoot))) "Undefined" "MultiplyWithRoot" 0 0))
  (Variables|Default|SetCurrentRoomSpawnPoint (Transformation|GetWorldLocation (Variables|/Game/PCG/BP_Room_BASE.BP_Room_BASE_C|GetEndPoint _returnvalue)))
  (for _index (range 0 14)
    (bind _returnvalue_2 (Game|SpawnActorfromClass (.OutItem (Utilities|Array|Random (Variables|Default|GetMiddleRooms))) (Math|Conversions|ToTransform(Vector) (Variables|Default|GetCurrentRoomSpawnPoint)) "Undefined" "MultiplyWithRoot" 0 0))
    (Variables|Default|SetCurrentRoomSpawnPoint (Transformation|GetWorldLocation (Variables|/Game/PCG/BP_Room_BASE.BP_Room_BASE_C|GetEndPoint _returnvalue_2))))
  (Game|SpawnActorfromClass "/Game/PCG/BP_EndRoom_A.BP_EndRoom_A_C" (Math|Conversions|ToTransform(Vector) (Variables|Default|GetCurrentRoomSpawnPoint)) "Undefined" "MultiplyWithRoot" 0 0))

(event Collision|EventActorBeginOverlap
  (params (OtherActor :type Actor%20Object%20Reference)))

(event EventTick
  (params (DeltaSeconds :type Float%20%28single-precision%29)))

(fn ConstructionScript)