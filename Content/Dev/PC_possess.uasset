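; Test player-controller Blueprint that toggles control between a third-person and a first-person character.
; On BeginPlay it spawns both characters near the world origin and stores their references.
; Pressing the 1 key flip-flops possession between them, removing the other character's Enhanced Input mapping context and adding the matching one.
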(event `self.ReceiveBeginPlay`
  (bind _returnvalue (`|SpawnActorFromClass` "/Game/TPCC/ThirdPerson/Blueprints/BP_ThirdPersonCharacter.BP_ThirdPersonCharacter_C" (`KismetMathLibrary.MakeTransform` (0.0 0.0 50.0)) "Undefined" "MultiplyWithRoot" null null))
  (set `self.cc01` _returnvalue)
  (bind _returnvalue_2 (`|SpawnActorFromClass` "/Game/FPCC/FirstPerson/Blueprints/BP_FirstPersonCharacter.BP_FirstPersonCharacter_C" (`KismetMathLibrary.MakeTransform` (0.0 50.0 50.0)) "Undefined" "MultiplyWithRoot" null null))
  (set `self.cc02` _returnvalue_2))

(event `Key|One`
  (params (Key :type "Key Structure"))
  (bind _returnvalue (`GameplayStatics.GetPlayerController` 0))
  (bind _returnvalue_2 (pcsubsystem `EnhancedInputLocalPlayerSubsystem` _returnvalue))
  (:`Pressed`
    (`/Engine/EditorBlueprintResources/StandardMacros.FlipFlop`
      (:`A`
        (message `EnhancedInputSubsystemInterface.RemoveMappingContext` _returnvalue_2 "/Game/FPCC/FirstPerson/Input/IMC_Default_FP.IMC_Default_FP" (struct))
        (`self.Possess` _returnvalue (`self.cc01`))
        (message `EnhancedInputSubsystemInterface.AddMappingContext` _returnvalue_2 "/Game/TPCC/ThirdPerson/Input/IMC_Default_TP.IMC_Default_TP" 0 (struct)))
      (:`B`
        (message `EnhancedInputSubsystemInterface.RemoveMappingContext` _returnvalue_2 "/Game/TPCC/ThirdPerson/Input/IMC_Default_TP.IMC_Default_TP" (struct))
        (`self.Possess` _returnvalue (`self.cc02`))
        (message `EnhancedInputSubsystemInterface.AddMappingContext` _returnvalue_2 "/Game/FPCC/FirstPerson/Input/IMC_Default_FP.IMC_Default_FP" 0 (struct))))))

(fn `UserConstructionScript`)