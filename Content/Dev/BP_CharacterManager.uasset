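; BP_CharacterManager is an actor that lets the player switch between a third-person and a first-person character.
; On BeginPlay it enables input on itself, spawns both characters side by side and keeps references to them.
; Pressing the 1 key drives a FlipFlop that has player controller 0 alternately possess the third-person and first-person pawns.
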(event `self.ReceiveBeginPlay`
  (`self.EnableInput` (`GameplayStatics.GetPlayerController` 0))
  (bind _returnvalue (`|SpawnActorFromClass` "/Game/TPCC/ThirdPerson/Blueprints/BP_ThirdPersonCharacter.BP_ThirdPersonCharacter_C" (`KismetMathLibrary.MakeTransform` (0.0 0.0 50.0)) "Undefined" "MultiplyWithRoot" null null))
  (set `self.CC1` _returnvalue)
  (bind _returnvalue_2 (`|SpawnActorFromClass` "/Game/FPCC/FirstPerson/Blueprints/BP_FirstPersonCharacter.BP_FirstPersonCharacter_C" (`KismetMathLibrary.MakeTransform` (0.0 50.0 50.0)) "Undefined" "MultiplyWithRoot" null null))
  (set `self.CC2` _returnvalue_2))

(event `Key|One`
  (params (Key :type "Key Structure"))
  (:`Pressed`
    (`/Engine/EditorBlueprintResources/StandardMacros.FlipFlop`
      (:`A`
        (`Controller.Possess` (`GameplayStatics.GetPlayerController` 0) (`self.CC1`))
        (`KismetSystemLibrary.Delay` 0.5))
      (:`B`
        (`Controller.Possess` (`GameplayStatics.GetPlayerController` 0) (`self.CC2`))))))

(fn `UserConstructionScript`)