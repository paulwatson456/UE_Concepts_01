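; PC_Possession is a player controller that switches the player between a first-person and a third-person pawn.
; On BeginPlay it spawns both pawns at fixed, offset locations and stores a reference to each.
; Key 1 drives a FlipFlop that alternately possesses each pawn through player controller 0, swapping the matching Enhanced Input mapping context on each switch.
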(event `self.ReceiveBeginPlay`
  (bind _returnvalue (`|SpawnActorFromClass` "/Game/Posession/BP_FirstPersonPosession.BP_FirstPersonPosession_C" (`KismetMathLibrary.MakeTransform` (0.0 40.0 0.0)) "Undefined" "MultiplyWithRoot" null null))
  (set `self.FP_CC` _returnvalue)
  (bind _returnvalue_2 (`|SpawnActorFromClass` "/Game/Posession/BP_ThirdPersonPossession.BP_ThirdPersonPossession_C" (`KismetMathLibrary.MakeTransform` (0.0 -40.0 0.0)) "Undefined" "MultiplyWithRoot" null null))
  (set `self.TP_CC` _returnvalue_2))

(event `Key|One`
  (params (Key :type "Key Structure"))
  (bind _returnvalue (`GameplayStatics.GetPlayerController` 0))
  (bind _returnvalue_2 (pcsubsystem `EnhancedInputLocalPlayerSubsystem` _returnvalue))
  (bind _returnvalue_3 (pcsubsystem `EnhancedInputLocalPlayerSubsystem` (`GameplayStatics.GetPlayerController` 0)))
  (:`Pressed`
    (`/Engine/EditorBlueprintResources/StandardMacros.FlipFlop`
      (:`A`
        (`self.Possess` _returnvalue (`self.FP_CC`))
        (`EnhancedInputSubsystemInterface.RemoveMappingContext` _returnvalue_2 "/Game/TPCC/ThirdPerson/Input/IMC_Default_TP.IMC_Default_TP" (struct))
        (`EnhancedInputSubsystemInterface.AddMappingContext` _returnvalue_3 "/Game/FPCC/FirstPerson/Input/IMC_Default_FP.IMC_Default_FP" 0 (struct)))
      (:`B`
        (`self.Possess` _returnvalue (`self.TP_CC`))
        (`EnhancedInputSubsystemInterface.RemoveMappingContext` _returnvalue_2 "/Game/FPCC/FirstPerson/Input/IMC_Default_FP.IMC_Default_FP" (struct))
        (`EnhancedInputSubsystemInterface.AddMappingContext` _returnvalue_3 "/Game/TPCC/ThirdPerson/Input/IMC_Default_TP.IMC_Default_TP" 0 (struct))))))

(fn `UserConstructionScript`)