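; BP_Marble_01 is a marble driven by Enhanced Input, with forward/back and left/right movement and a jump.
; BeginPlay adds the MC_MyContext mapping context to player controller 0.
; Move actions apply scaled acceleration-change forces to the Sphere along the DefaultSceneRoot forward and right vectors.
; Jump applies a one-shot, mass-dependent upward impulse along the root's up vector, with no grounded check.
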(event `self.ReceiveBeginPlay`
  (`EnhancedInputSubsystemInterface.AddMappingContext` (pcsubsystem `EnhancedInputLocalPlayerSubsystem` (`GameplayStatics.GetPlayerController` 0)) "/Game/CC_Input/MC_MyContext.MC_MyContext" 0 (struct)))

(event `EnhancedInput|/Game/CC_Input/MyInputActions/IA_MyMoveFB`
  (params (ActionValue :type "Float (double-precision)") (ElapsedSeconds :type "Float (double-precision)") (TriggeredSeconds :type "Float (double-precision)") (InputAction :type "InputAction Object Reference" :default "/Game/CC_Input/MyInputActions/IA_MyMoveFB.IA_MyMoveFB"))
  (:`Triggered`
    (`PrimitiveComponent.AddForce` (`self.Sphere`) (* (`SceneComponent.GetForwardVector` (`self.DefaultSceneRoot`)) (* ActionValue 1000.0)) "None" true)))

(event `EnhancedInput|/Game/CC_Input/MyInputActions/IA_MyMoveLR`
  (params (ActionValue :type "Float (double-precision)") (ElapsedSeconds :type "Float (double-precision)") (TriggeredSeconds :type "Float (double-precision)") (InputAction :type "InputAction Object Reference" :default "/Game/CC_Input/MyInputActions/IA_MyMoveLR.IA_MyMoveLR"))
  (:`Triggered`
    (`PrimitiveComponent.AddForce` (`self.Sphere`) (* (`SceneComponent.GetRightVector` (`self.DefaultSceneRoot`)) (* ActionValue 1000.0)) "None" true)))

(event `EnhancedInput|/Game/CC_Input/MyInputActions/IA_MyJump`
  (params (ActionValue :type Boolean) (ElapsedSeconds :type "Float (double-precision)") (TriggeredSeconds :type "Float (double-precision)") (InputAction :type "InputAction Object Reference" :default "/Game/CC_Input/MyInputActions/IA_MyJump.IA_MyJump"))
  (:`Started`
    (`PrimitiveComponent.AddImpulse` (`self.Sphere`) (* (`SceneComponent.GetUpVector` (`self.DefaultSceneRoot`)) 600.0) "None" false)))

(fn `UserConstructionScript`)