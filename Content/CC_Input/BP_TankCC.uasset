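; Player-controlled tank that drives, turns, rotates its turret and fires through Enhanced Input, adding the IM_Tank mapping context on BeginPlay.
; Input moves the actor along BodyDirection's forward vector and yaws it, using fixed per-trigger steps without sweep or delta-time scaling.
; The turret yaws locally on its own input.
; Firing spawns BP_TankGun_01 at GunDirection's location with the turret's world rotation.
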(event `self.ReceiveBeginPlay`
  (`EnhancedInputSubsystemInterface.AddMappingContext` (pcsubsystem `EnhancedInputLocalPlayerSubsystem` (`GameplayStatics.GetPlayerController` 0)) "/Game/CC_Input/MyInputActions/TankActions/IM_Tank.IM_Tank" 0 (struct)))

(event `EnhancedInput|/Game/CC_Input/MyInputActions/TankActions/IA_Tank_FB`
  (params (ActionValue :type "Float (double-precision)") (ElapsedSeconds :type "Float (double-precision)") (TriggeredSeconds :type "Float (double-precision)") (InputAction :type "InputAction Object Reference" :default "/Game/CC_Input/MyInputActions/TankActions/IA_Tank_FB.IA_Tank_FB"))
  (:`Triggered`
    (`self.K2_AddActorWorldOffset` (* (`SceneComponent.GetForwardVector` (`self.BodyDirection`)) (* ActionValue 3.0)))))

(event `EnhancedInput|/Game/CC_Input/MyInputActions/TankActions/IA_Tank_R_LR`
  (params (ActionValue :type "Float (double-precision)") (ElapsedSeconds :type "Float (double-precision)") (TriggeredSeconds :type "Float (double-precision)") (InputAction :type "InputAction Object Reference" :default "/Game/CC_Input/MyInputActions/TankActions/IA_Tank_R_LR.IA_Tank_R_LR"))
  (:`Triggered`
    (`self.K2_AddActorWorldRotation` (`KismetMathLibrary.MakeRotator` 0.0 0.0 (/ ActionValue 2.0)))))

(event `EnhancedInput|/Game/CC_Input/MyInputActions/TankActions/IA_TankTurret_R_LR`
  (params (ActionValue :type "Vector2D Structure") (ElapsedSeconds :type "Float (double-precision)") (TriggeredSeconds :type "Float (double-precision)") (InputAction :type "InputAction Object Reference" :default "/Game/CC_Input/MyInputActions/TankActions/IA_TankTurret_R_LR.IA_TankTurret_R_LR"))
  (:`Triggered`
    (`SceneComponent.K2_AddLocalRotation` (`self.Turret`) (`KismetMathLibrary.MakeRotator` 0.0 0.0 ActionValue_X) false false)))

(event `EnhancedInput|/Game/CC_Input/MyInputActions/TankActions/IA_TankFire`
  (params (ActionValue :type Boolean) (ElapsedSeconds :type "Float (double-precision)") (TriggeredSeconds :type "Float (double-precision)") (InputAction :type "InputAction Object Reference" :default "/Game/CC_Input/MyInputActions/TankActions/IA_TankFire.IA_TankFire"))
  (:`Started`
    (`|SpawnActorFromClass` "/Game/CC_Input/BP_TankGun_01.BP_TankGun_01_C" (`KismetMathLibrary.MakeTransform` (`SceneComponent.K2_GetComponentLocation` (`self.GunDirection`)) (`SceneComponent.K2_GetComponentRotation` (`self.Turret`))) "Undefined" "MultiplyWithRoot" null null)))

(fn `UserConstructionScript`)