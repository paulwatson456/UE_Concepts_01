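; Player character for a 2.5D game, with Enhanced Input movement, jumping, turning, dashing and shooting.
; Forward/back input ignores control yaw while left/right follows it, and a general movement axis rotates the capsule.
; Right mouse runs a Dash timeline that offsets the actor along its normalized velocity without sweeping.
; Left mouse spawns BP_Bullet_01 at the Nose component's location and rotation.
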(event `self.ReceiveBeginPlay`
  (`EnhancedInputSubsystemInterface.AddMappingContext` (pcsubsystem `EnhancedInputLocalPlayerSubsystem` (`GameplayStatics.GetPlayerController` 0)) "/Game/CC_Input/MC_MyContext.MC_MyContext" 0 (struct)))

(event `EnhancedInput|/Game/CC_Input/MyInputActions/IA_MyMoveFB`
  (params (ActionValue :type "Float (double-precision)") (ElapsedSeconds :type "Float (double-precision)") (TriggeredSeconds :type "Float (double-precision)") (InputAction :type "InputAction Object Reference" :default "/Game/CC_Input/MyInputActions/IA_MyMoveFB.IA_MyMoveFB"))
  (bind _returnvalue_roll (`KismetMathLibrary.BreakRotator` (`self.GetControlRotation`)))
  (:`Triggered`
    (`self.AddMovementInput` (`KismetMathLibrary.GetForwardVector` (`KismetMathLibrary.MakeRotator` _returnvalue_roll)) ActionValue)))

(event `EnhancedInput|/Game/CC_Input/MyInputActions/IA_MyMoveLR`
  (params (ActionValue :type "Float (double-precision)") (ElapsedSeconds :type "Float (double-precision)") (TriggeredSeconds :type "Float (double-precision)") (InputAction :type "InputAction Object Reference" :default "/Game/CC_Input/MyInputActions/IA_MyMoveLR.IA_MyMoveLR"))
  (bind (_returnvalue_roll _returnvalue_pitch _returnvalue_yaw) (`KismetMathLibrary.BreakRotator` (`self.GetControlRotation`)))
  (:`Triggered`
    (`self.AddMovementInput` (`KismetMathLibrary.GetRightVector` (`KismetMathLibrary.MakeRotator` _returnvalue_roll 0.0 _returnvalue_yaw)) ActionValue)))

(event `EnhancedInput|/Game/CC_Input/MyInputActions/IA_MyJump`
  (params (ActionValue :type Boolean) (ElapsedSeconds :type "Float (double-precision)") (TriggeredSeconds :type "Float (double-precision)") (InputAction :type "InputAction Object Reference" :default "/Game/CC_Input/MyInputActions/IA_MyJump.IA_MyJump"))
  (:`Triggered`
    (`self.Jump`))
  (:`Completed`
    (`self.StopJumping`)))

(event `Key|RightMouseButton`
  (params (Key :type "Key Structure"))
  (:`Pressed`
    (`Timeline|Dash` :!via `PlayFromStart`
      (:`Update`
        (`self.K2_AddActorWorldOffset` (* (`KismetMathLibrary.Normal` (`CharacterMovementComponent.GetLastUpdateVelocity` (`self.CharacterMovement`))) 10.0))))))

(event `EnhancedInput|/Game/CC_Input/MyInputActions/IA_MyGeneralMovement`
  (params (ActionValue :type "Vector2D Structure") (ElapsedSeconds :type "Float (double-precision)") (TriggeredSeconds :type "Float (double-precision)") (InputAction :type "InputAction Object Reference" :default "/Game/CC_Input/MyInputActions/IA_MyGeneralMovement.IA_MyGeneralMovement"))
  (:`Triggered`
    (`SceneComponent.K2_AddLocalRotation` (`self.CapsuleComponent`) (`KismetMathLibrary.MakeRotator` 0.0 0.0 (* ActionValue_X 2.0)) false false)))

(event `Key|LeftMouseButton`
  (params (Key :type "Key Structure"))
  (bind _nose (`self.Nose`))
  (:`Pressed`
    (`|SpawnActorFromClass` "/Game/CC_Input/BP_Bullet_01.BP_Bullet_01_C" (`KismetMathLibrary.MakeTransform` (`SceneComponent.K2_GetComponentLocation` _nose) (`SceneComponent.K2_GetComponentRotation` _nose)) "Undefined" "MultiplyWithRoot" null null)))

(fn `UserConstructionScript`)