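; Player character Blueprint for a 2.5D setup, with movement and jumping driven by Enhanced Input.
; BeginPlay adds the MC_MyContext mapping context to the first player controller.
; The forward/back and left/right actions add movement along the Cube component's forward and right vectors rather than the control rotation, and the jump action starts and stops jumping.
; Control-rotation vector nodes, a relative-location setter and an empty RotationRate event are inactive leftovers.
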(event `self.ReceiveBeginPlay`
  (`EnhancedInputSubsystemInterface.AddMappingContext` (pcsubsystem `EnhancedInputLocalPlayerSubsystem` (`GameplayStatics.GetPlayerController` 0)) "/Game/CC_Input/MC_MyContext.MC_MyContext" 0 (struct)))

(event `EnhancedInput|/Game/CC_Input/MyInputActions/IA_MyMoveFB`
  (params (ActionValue :type "Float (double-precision)") (ElapsedSeconds :type "Float (double-precision)") (TriggeredSeconds :type "Float (double-precision)") (InputAction :type "InputAction Object Reference" :default "/Game/CC_Input/MyInputActions/IA_MyMoveFB.IA_MyMoveFB"))
  (:`Triggered`
    (`self.AddMovementInput` (`SceneComponent.GetForwardVector` (`self.Cube`)) ActionValue)))

(event `EnhancedInput|/Game/CC_Input/MyInputActions/IA_MyMoveLR`
  (params (ActionValue :type "Float (double-precision)") (ElapsedSeconds :type "Float (double-precision)") (TriggeredSeconds :type "Float (double-precision)") (InputAction :type "InputAction Object Reference" :default "/Game/CC_Input/MyInputActions/IA_MyMoveLR.IA_MyMoveLR"))
  (:`Triggered`
    (`self.AddMovementInput` (`SceneComponent.GetRightVector` (`self.Cube`)) ActionValue)))

(event `InputVectorAxis|RotationRate`
  (params (AxisValue :type "Vector Structure")))

(event `EnhancedInput|/Game/CC_Input/MyInputActions/IA_MyJump`
  (params (ActionValue :type Boolean) (ElapsedSeconds :type "Float (double-precision)") (TriggeredSeconds :type "Float (double-precision)") (InputAction :type "InputAction Object Reference" :default "/Game/CC_Input/MyInputActions/IA_MyJump.IA_MyJump"))
  (:`Triggered`
    (`self.Jump`))
  (:`Completed`
    (`self.StopJumping`)))

(fn `UserConstructionScript`)