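; Movement pawn prototype with Enhanced Input walking, jump and a right-mouse timeline dash, moved by unswept offsets and impulses.
; Forward and right inputs, halved when airborne, combine into a direction vector that drives the dash, jump drift and cube rotation.
; Tick eases the cube toward that direction and sets Grounded from a downward trace distance.
; Jump applies impulses during the first 0.15 seconds of input, without checking Grounded.
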(event `self.ReceiveTick`
  (params (DeltaSeconds :type "Float (single-precision)"))
  (bind _bodycol (`self.BodyCOL`))
  (bind _returnvalue (`SceneComponent.K2_GetComponentLocation` _bodycol))
  (bind (_returnvalue_x _returnvalue_y _returnvalue_z) (`KismetMathLibrary.BreakVector` (`SceneComponent.K2_GetComponentLocation` _bodycol)))
  (`SceneComponent.K2_SetRelativeRotation` (`self.Cube`) (`KismetMathLibrary.RInterpTo` (`SceneComponent.RelativeRotation` (`self.Cube`)) (`self.DirectionROT`) DeltaSeconds 10.0) false false)
  (bind _outhit (`KismetSystemLibrary.LineTraceSingle` :`Start` _returnvalue :`End` (`KismetMathLibrary.MakeVector` _returnvalue_x _returnvalue_y (- _returnvalue_z 500.0)) :`TraceChannel` "TraceTypeQuery1" :`DrawDebugType` "ForOneFrame"))
  (if (< (`KismetMathLibrary.Vector_Distance` _returnvalue (`.Location` (`GameplayStatics.BreakHitResult` _outhit))) 53.0)
    (set `self.Grounded?` true)
    (else
      (set `self.Grounded?` false))))

(event `self.ReceiveBeginPlay`
  (`EnhancedInputSubsystemInterface.AddMappingContext` (pcsubsystem `EnhancedInputLocalPlayerSubsystem` (`GameplayStatics.GetPlayerController` 0)) "/Game/CC_Input/MC_MyContext.MC_MyContext" 0 (struct)))

(event `EnhancedInput|/Game/CC_Input/MyInputActions/IA_MyMoveFB`
  (params (ActionValue :type "Float (double-precision)") (ElapsedSeconds :type "Float (double-precision)") (TriggeredSeconds :type "Float (double-precision)") (InputAction :type "InputAction Object Reference" :default "/Game/CC_Input/MyInputActions/IA_MyMoveFB.IA_MyMoveFB"))
  (bind _returnvalue (* (`SceneComponent.GetForwardVector` (`self.F-Direction`)) (* ActionValue (`self.MovementSpeed`))))
  (:`Triggered`
    (if (`self.Grounded?`)
      (set `self.FB_Direction` _returnvalue)
      (else
        (set `self.FB_Direction` (/ _returnvalue 2.0))))
    (`self.K2_AddActorWorldOffset` (`self.FB_Direction`))
    (bind _output_get (set `self.PawnVectorDirection` (+ (`self.FB_Direction`) (`self.LR_Direction`)) :!label _label))
    (set `self.DirectionROT` (`KismetMathLibrary.Conv_VectorToRotator` _output_get)))
  (:`Started`
    (`self.Rotate towards direction`))
  (:`Completed`
    (set `self.FB_Direction` (0.0 0.0 0.0))))

(event `EnhancedInput|/Game/CC_Input/MyInputActions/IA_MyMoveLR`
  (params (ActionValue :type "Float (double-precision)") (ElapsedSeconds :type "Float (double-precision)") (TriggeredSeconds :type "Float (double-precision)") (InputAction :type "InputAction Object Reference" :default "/Game/CC_Input/MyInputActions/IA_MyMoveLR.IA_MyMoveLR"))
  (bind _returnvalue (* (`SceneComponent.GetRightVector` (`self.F-Direction`)) (* ActionValue (`self.MovementSpeed`))))
  (:`Triggered`
    (if (`self.Grounded?`)
      (set `self.LR_Direction` _returnvalue)
      (else
        (set `self.LR_Direction` (/ _returnvalue 2.0))))
    (`self.K2_AddActorWorldOffset` (`self.LR_Direction`))
    (goto _label))
  (:`Started`
    (`self.Rotate towards direction`))
  (:`Completed`
    (set `self.LR_Direction` (0.0 0.0 0.0))))

(event `EnhancedInput|/Game/CC_Input/MyInputActions/IA_MyJump`
  (params (ActionValue :type Boolean) (ElapsedSeconds :type "Float (double-precision)") (TriggeredSeconds :type "Float (double-precision)") (InputAction :type "InputAction Object Reference" :default "/Game/CC_Input/MyInputActions/IA_MyJump.IA_MyJump"))
  (bind (_pawnvectordirection_x _pawnvectordirection_y) (`KismetMathLibrary.BreakVector` (`self.PawnVectorDirection`)))
  (:`Triggered`
    (set `self.Grounded?` false)
    (if (not (> TriggeredSeconds 0.15))
      (`PrimitiveComponent.AddImpulse` (`self.BodyCOL`) (`KismetMathLibrary.MakeVector` (* _pawnvectordirection_x 5.0) (* _pawnvectordirection_y 5.0) 40.0) "None" true))))

(event `Key|RightMouseButton`
  (params (Key :type "Key Structure"))
  (:`Pressed`
    (`Timeline|Timeline` :!via `PlayFromStart`
      (:`Update`
        (`SceneComponent.K2_AddWorldOffset` (`self.BodyCOL`) (* (`self.PawnVectorDirection`) 5.0) false false)))))

(event `Rotate towards direction`
  (bind (_direction _newtrack_0) (`Timeline|Rotation` :!via `PlayFromStart`)
    (:`Update`
      (`SceneComponent.K2_SetRelativeRotation` (`self.Cube`) (`KismetMathLibrary.RLerp` (`SceneComponent.RelativeRotation` (`self.Cube`)) (`self.DirectionROT`) _newtrack_0 true) false false))))

(fn `UserConstructionScript`)