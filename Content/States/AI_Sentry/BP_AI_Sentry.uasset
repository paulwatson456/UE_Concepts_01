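; AI sentry camera that patrols, tracks the player and raises an alert, with a status light for each state.
; A looping timeline swings the camera head through rotation points until a vision cone overlap stops it and starts per-tick tracking of the player.
; Once a dot-product facing check passes, a one-second timer confirms the sighting and notifies all I_AlertManager actors.
; Ending the overlap resumes patrol and resets the alert gate.
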(event `self.VisionCone.OnComponentBeginOverlap`
  (params (OverlappedComponent :type "PrimitiveComponent Object Reference") (OtherActor :type "Actor Object Reference") (OtherComp :type "PrimitiveComponent Object Reference") (OtherBodyIndex :type Integer) (bFromSweep :type Boolean) (SweepResult :type "HitResult Structure (by ref)"))
  (`self.StopPatrolMovement`)
  (set `self.PLayerSeen?` true)
  (`PrimitiveComponent.SetMaterial` (`self.AlertStatus`) 0 "/Game/States/AI_Sentry/M_AlertLightState_Orange.M_AlertLightState_Orange"))

(event `self.ReceiveBeginPlay`
  (`self.Patrol`))

(event `Patrol`
  ;[0.1164 0.05241 1] Patrol State
  (bind (_direction _newtrack_0) (`Timeline|PatrolRotation` :!via `PlayFromStart` :!label _label)
    (:`Update`
      (`SceneComponent.K2_SetRelativeRotation` (`self.Mesh_CameraHead`) (`KismetMathLibrary.RLerp` (`self.CurrentROT`) (`|GetArrayItem` (`self.RotationPoints`) (`self.PositionSelection`)) _newtrack_0) false false))
    (:`Finished`
      (bind _output_get (set `self.PositionSelection` (+ (`self.PositionSelection`) 1)))
      (if (>= _output_get (`KismetArrayLibrary.Array_Length` (`self.RotationPoints`)))
        (set `self.PositionSelection` 0)
        (set `self.CurrentROT` (`SceneComponent.RelativeRotation` (`self.Mesh_CameraHead`)))
        (`self.Patrol`)
        (else
          (set `self.CurrentROT` (`SceneComponent.RelativeRotation` (`self.Mesh_CameraHead`)))
          (`self.Patrol`))))))

(event `StopPatrolMovement`
  ;[0.1164 0.05241 1] Patrol State
  (goto _label :!via `Stop`))

(event `self.VisionCone.OnComponentEndOverlap`
  (params (OverlappedComponent :type "PrimitiveComponent Object Reference") (OtherActor :type "Actor Object Reference") (OtherComp :type "PrimitiveComponent Object Reference") (OtherBodyIndex :type Integer))
  (set `self.PLayerSeen?` false)
  (set `self.CurrentROT` (`SceneComponent.RelativeRotation` (`self.Mesh_CameraHead`)))
  (set `self.PositionSelection` 0)
  (`self.Patrol`)
  (`self.ReduceAlert`)
  (`PrimitiveComponent.SetMaterial` (`self.AlertStatus`) 0 "/Game/States/AI_Sentry/M_AlertLightState_GREEN.M_AlertLightState_GREEN"))

(event `self.ReceiveTick`
  (params (DeltaSeconds :type "Float (single-precision)"))
  (bind _mesh_camerahead (`self.Mesh_CameraHead`))
  ;[1 0.5668 0.003265] CautionState
  (if (`self.PLayerSeen?`)
    (`SceneComponent.K2_SetRelativeRotation` (`self.Mesh_CameraHead`) (`KismetMathLibrary.RInterpTo_Constant` (`SceneComponent.K2_GetComponentRotation` (`self.Mesh_CameraHead`)) (`KismetMathLibrary.FindLookAtRotation` (`SceneComponent.K2_GetComponentLocation` (`self.Mesh_CameraHead`)) (`self.K2_GetActorLocation` (`GameplayStatics.GetPlayerPawn` 0))) DeltaSeconds 60.0) false false)
    (if (> (`KismetMathLibrary.Dot_VectorVector` (`KismetMathLibrary.GetDirectionUnitVector` (`SceneComponent.K2_GetComponentLocation` _mesh_camerahead) (`self.K2_GetActorLocation` (`GameplayStatics.GetPlayerPawn` 0))) (`SceneComponent.GetForwardVector` _mesh_camerahead)) 0.8)
      (`/Engine/EditorBlueprintResources/StandardMacros.DoOnce` false :!label _label_2
        (:`Completed`
          (`KismetSystemLibrary.K2_SetTimerDelegate` (delegate `PlayerSeen`) 1.0))))))

(event `ReduceAlert`
  (goto _label_2 :!via `Reset`))

(event `PlayerSeen`
  (if (`self.PLayerSeen?`)
    (`self.AlertEvent`)))

(event `AlertEvent`
  ;[1 0 0.02832] AlertState
  (`PrimitiveComponent.SetMaterial` (`self.AlertStatus`) 0 "/Game/States/AI_Sentry/M_AlertLightState_RED.M_AlertLightState_RED")
  (bind _outactors (`GameplayStatics.GetAllActorsWithInterface` "/Game/States/AI_Sentry/I_AlertManager.I_AlertManager_C"))
  (for _array_element _outactors
    (message `/Game/States/AI_Sentry/I_AlertManager.EnemySighted` _array_element)))

(event `self.CheckStatus`
  (`self.SendStatus`))

(fn `SendStatus`
  (returns (`CanStillSeePLayer?` :type Boolean))
  (return (`self.PLayerSeen?`)))

(fn `UserConstructionScript`)