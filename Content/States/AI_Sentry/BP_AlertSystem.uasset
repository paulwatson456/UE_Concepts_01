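; Alert manager for AI sentries that moves the game through spotted, caution and no-alert states when the player is seen.
; A sighting shows the spotted widget and broadcasts activation to every I_AlertComms actor.
; After a delay it polls those actors, re-entering alert if any still sees the player, otherwise showing the caution widget.
; A caution timer then removes that widget and broadcasts deactivation through the same interface.
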(event `self.PlayerInView`
  (`/Engine/EditorBlueprintResources/StandardMacros.IsValid` (`self.CautionUI`)
    (:`Is Valid`
      (`Widget.RemoveFromParent` (`self.CautionUI`)))
    (:`Is Not Valid`
      _))
  (bind _returnvalue (`|CreateWidget` "/Game/States/AI_Sentry/WBP_SpottedAlert.WBP_SpottedAlert_C"))
  (`/Engine/EditorBlueprintResources/StandardMacros.IsValid` (`self.SpottedUI`)
    (:`Is Valid`
      _)
    (:`Is Not Valid`
      (bind _output_get (set `self.SpottedUI` _returnvalue))))
  (`UserWidget.AddToViewport` _output_get 0)
  (`self.Alert ON`))

(event `Alert ON`
  ;[1 0.0877 0.8282] Alert BP
  (`self.SendAlertMessage`)
  (`KismetSystemLibrary.Delay` 2.0)
  (`self.CheckStatusOfAI_Sentrys`))

(event `SendAlertMessage`
  ;[1 0.0877 0.8282] Alert BP
  (bind _outactors (`GameplayStatics.GetAllActorsWithInterface` "/Game/States/AI_Sentry/I_AlertComms.I_AlertComms_C"))
  (for _array_element _outactors
    (message `/Game/States/AI_Sentry/I_AlertComms.AlertSystemActivated` _array_element)))

(event `CheckStatusOfAI_Sentrys`
  ;[1 0.0877 0.8282] Alert BP
  (bind _outactors (`GameplayStatics.GetAllActorsWithInterface` "/Game/States/AI_Sentry/I_AlertComms.I_AlertComms_C"))
  (for _array_element _outactors
    (bind _canaisentryseeplayer_ (message `/Game/States/AI_Sentry/I_AlertComms.PlayerViewStatusCheck` _array_element))
    (`KismetArrayLibrary.Array_Add` (`self.CanSentrysSeePlayer?`) _canaisentryseeplayer_))
  (`self.StatusCheckResult`))

(event `StatusCheckResult`
  ;[1 0.0877 0.8282] Alert BP
  (if (`KismetArrayLibrary.Array_Contains` (`self.CanSentrysSeePlayer?`) true)
    (`KismetArrayLibrary.Array_Clear` (`self.CanSentrysSeePlayer?`))
    (`self.PlayerInView`)
    (else
      (`KismetArrayLibrary.Array_Clear` (`self.CanSentrysSeePlayer?`))
      (`self.Caution`))))

(event `Caution`
  (`/Engine/EditorBlueprintResources/StandardMacros.IsValid` (`self.SpottedUI`)
    (:`Is Valid`
      (`Widget.RemoveFromParent` (`self.SpottedUI`)))
    (:`Is Not Valid`
      _))
  (bind _returnvalue (`|CreateWidget` "/Game/States/AI_Sentry/WBP_CautionAlert.WBP_CautionAlert_C"))
  (bind _output_get (set `self.CautionUI` _returnvalue))
  (`UserWidget.AddToViewport` _output_get 0)
  (`self.SearchingFor Player`))

(event `SearchingFor Player`
  ;[1 1 1] Caution State
  (`KismetSystemLibrary.K2_SetTimerDelegate` (delegate `SendDeactivateAlertMessage`) 3.0))

(event `SendDeactivateAlertMessage`
  ;[1 1 1] Caution State
  (`self.TransitionNoAlert`))

(event `TransitionNoAlert`
  (`/Engine/EditorBlueprintResources/StandardMacros.IsValid` (`self.CautionUI`)
    (:`Is Valid`
      (`Widget.RemoveFromParent` (`self.CautionUI`))
      (`self.AlertOFF`))))

(event `AlertOFF`
  ;[1 1 1] No Slert State
  (bind _outactors (`GameplayStatics.GetAllActorsWithInterface` "/Game/States/AI_Sentry/I_AlertComms.I_AlertComms_C"))
  (for _array_element _outactors
    (message `/Game/States/AI_Sentry/I_AlertComms.AlertSystemDeacivated` _array_element)))

(fn `PlayerViewStatusCheck`
  (returns (`CanAISentrySeePlayer?` :type Boolean))
  (return false))

(fn `UserConstructionScript`)