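; Sentry AI that sweeps a vision cone through rotation points with a looping timeline, though BeginPlay calls an empty Patrol event.
; Any cone overlap halts the sweep, turns the light orange and makes Tick yaw toward the player.
; Once roughly facing them, a one-second timer turns it red and alerts I_SentryComms actors if overlap persists.
; Ending overlap turns it green, sends deactivation and resumes the sweep.
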(event `Patrol`
  ;[0.1832 0.2887 1] Patrol Start
)

(event `self.ReceiveBeginPlay`
  (`self.Patrol`))

(event `Move`
  ;[0.1832 0.2887 1] Patrol Functionlality
  (bind (_direction _newtrack_0) (`Timeline|Rotation` :!via `PlayFromStart` :!label _label)
    (:`Update`
      (`SceneComponent.K2_SetRelativeRotation` (`self.Cube`) (`KismetMathLibrary.RLerp` (`self.CurrentROT`) (`|GetArrayItem` (`self.RotationPoints`) (`self.PositionSelection`)) _newtrack_0) false false))
    (:`Finished`
      (bind _output_get (set `self.PositionSelection` (+ (`self.PositionSelection`) 1)))
      (if (>= _output_get (`KismetArrayLibrary.Array_Length` (`self.RotationPoints`)))
        (set `self.PositionSelection` 0)
        (set `self.CurrentROT` (`SceneComponent.RelativeRotation` (`self.Cube`)))
        (`self.Move`)
        (else
          (set `self.CurrentROT` (`SceneComponent.RelativeRotation` (`self.Cube`)))
          (`self.Move`))))))

(event `StopMove`
  ;[0.1832 0.2887 1] Patrol Functionlality
  (goto _label :!via `Stop`))

(event `PlayerSeen`
  ;[1 0 0] Alert State Start
  (`PrimitiveComponent.SetMaterial` (`self.State`) 0 "/Game/States/AI_Sentry/M_Light_Red.M_Light_Red")
  (`self.Alert Action`))

(event `self.VisionCone.OnComponentBeginOverlap`
  (params (OverlappedComponent :type "PrimitiveComponent Object Reference") (OtherActor :type "Actor Object Reference") (OtherComp :type "PrimitiveComponent Object Reference") (OtherBodyIndex :type Integer) (bFromSweep :type Boolean) (SweepResult :type "HitResult Structure (by ref)"))
  (set `self.PlayerSeen?` true)
  (`self.StopMove`)
  (`PrimitiveComponent.SetMaterial` (`self.State`) 0 "/Game/States/AI_Sentry/M_Light_Orange.M_Light_Orange"))

(event `self.VisionCone.OnComponentEndOverlap`
  (params (OverlappedComponent :type "PrimitiveComponent Object Reference") (OtherActor :type "Actor Object Reference") (OtherComp :type "PrimitiveComponent Object Reference") (OtherBodyIndex :type Integer))
  (set `self.PlayerSeen?` false)
  (set `self.CurrentROT` (`SceneComponent.RelativeRotation` (`self.Cube`)))
  (set `self.PositionSelection` 0)
  (`self.ReduceAlert`)
  (`PrimitiveComponent.SetMaterial` (`self.State`) 0 "/Game/States/AI_Sentry/M_Light_Green.M_Light_Green")
  (`self.Move`))

(event `Alert Action`
  (bind _outactors (`GameplayStatics.GetAllActorsWithInterface` "/Game/States/AI_Sentry/I_SentryComms.I_SentryComms_C"))
  (for _array_element _outactors
    (message `/Game/States/AI_Sentry/I_SentryComms.AlertStateActivate` _array_element)))

(event `ReduceAlert`
  (`self.ResetPLayerSeen`)
  (bind _outactors (`GameplayStatics.GetAllActorsWithInterface` "/Game/States/AI_Sentry/I_SentryComms.I_SentryComms_C"))
  (for _array_element _outactors
    (message `/Game/States/AI_Sentry/I_SentryComms.AlertDeactivate` _array_element)))

(event `self.ReceiveTick`
  (params (DeltaSeconds :type "Float (single-precision)"))
  (bind _cube (`self.Cube`))
  (bind (_returnvalue_roll _returnvalue_pitch _returnvalue_yaw) (`KismetMathLibrary.BreakRotator` (`KismetMathLibrary.RInterpTo_Constant` (`SceneComponent.K2_GetComponentRotation` (`self.Cube`)) (`KismetMathLibrary.FindLookAtRotation` (`SceneComponent.K2_GetComponentLocation` (`self.Cube`)) (`self.K2_GetActorLocation` (`GameplayStatics.GetPlayerPawn` 0))) DeltaSeconds 70.0)))
  ;[1 0.3665 0] Alerted To Movement Functionality
  (if (`self.PlayerSeen?`)
    (`SceneComponent.K2_SetRelativeRotation` (`self.Cube`) (`KismetMathLibrary.MakeRotator` 0.0 0.0 _returnvalue_yaw) false false)
    (if (> (`KismetMathLibrary.Dot_VectorVector` (`KismetMathLibrary.GetDirectionUnitVector` (`SceneComponent.K2_GetComponentLocation` _cube) (`self.K2_GetActorLocation` (`GameplayStatics.GetPlayerPawn` 0))) (`SceneComponent.GetForwardVector` _cube)) 0.8)
      (`/Engine/EditorBlueprintResources/StandardMacros.DoOnce` false :!label _label_2
        (:`Completed`
          (bind _returnvalue (`KismetSystemLibrary.K2_SetTimerDelegate` (delegate `StartAlertState`) 1.0))
          (set `self.AlertTimerHandle` _returnvalue))))))

(event `ResetPLayerSeen`
  ;[1 0.3665 0] Alerted To Movement Functionality
  (goto _label_2 :!via `Reset`))

(event `StartAlertState`
  ;[1 0.3665 0] Alerted To Movement Functionality
  (if (`self.PlayerSeen?`)
    (`self.PlayerSeen`)))

(fn `UserConstructionScript`)