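; Defence door in the AI sentry area that opens on BeginPlay and on alert deactivation, and closes when the alert state activates.
; Separate open and close timelines lerp the door mesh's relative location toward its open or closed position.
; Each move stops the opposing timeline and starts from the mesh's current location, so a mid-travel reversal does not snap.
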(event `self.ReceiveBeginPlay`
  (`self.DoorOpen`))

(event `/Game/States/AI_Sentry/I_SentryComms.AlertDeactivate`
  (`self.DoorOpen`))

(event `/Game/States/AI_Sentry/I_SentryComms.AlertStateActivate`
  (`self.DoorClose`))

(event `StopClose`
  (bind (_direction _newtrack_0) (`Timeline|DoorCloseTime` :!via `Stop` :!label _label)
    (:`Update`
      (`SceneComponent.K2_SetRelativeLocation` (`self.DoorMesh`) (`KismetMathLibrary.VLerp` (`self.CurrentLOC`) (`self.CloseLOC`) _newtrack_0) false false))))

(event `DoorClose`
  (`self.StopOpen`)
  (set `self.CurrentLOC` (`SceneComponent.RelativeLocation` (`self.DoorMesh`)))
  (goto _label :!via `PlayFromStart`))

(event `DoorOpen`
  (`self.StopClose`)
  (set `self.CurrentLOC` (`SceneComponent.RelativeLocation` (`self.DoorMesh`)))
  (bind (_direction _newtrack_0) (`Timeline|DooCloseTime` :!via `PlayFromStart` :!label _label_2)
    (:`Update`
      (`SceneComponent.K2_SetRelativeLocation` (`self.DoorMesh`) (`KismetMathLibrary.VLerp` (`self.CurrentLOC`) (`self.OpenLOC`) _newtrack_0) false false))))

(event `StopOpen`
  (goto _label_2 :!via `Stop`))

(fn `UserConstructionScript`)