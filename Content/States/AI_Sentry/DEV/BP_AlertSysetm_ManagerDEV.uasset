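; Development alert manager for AI sentries that tracks whether any sentry can still see the player.
; EnemySighted polls every I_AlertManagerDEV actor for status and repeats each second while any reports true; otherwise it only prints all clear.
; EnemyLost broadcasts deactivation through the same interface.
; The activation broadcast and delayed EnemyLost timer are disconnected, AlertSystemON and CheckStatus are empty, and SendStatus returns false.
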(event `/Game/States/AI_Sentry/DEV/I_AlertManagerDEV.EnemySighted`
  ;[1 0.01372 0.8946] Comment
  (`self.Check status of sentrys`))

(event `EnemyLost`
  ;[1 0.01372 0.8946] Comment
  (bind _outactors (`GameplayStatics.GetAllActorsWithInterface` "/Game/States/AI_Sentry/DEV/I_AlertManagerDEV.I_AlertManagerDEV_C"))
  (for _array_element _outactors
    (message `/Game/States/AI_Sentry/DEV/I_AlertManagerDEV.AlertSystemDeactivated` _array_element)))

(event `Check status of sentrys`
  ;[1 0.01372 0.8946] Comment
  (bind _outactors (`GameplayStatics.GetAllActorsWithInterface` "/Game/States/AI_Sentry/DEV/I_AlertManagerDEV.I_AlertManagerDEV_C"))
  (for _array_element _outactors
    (bind _canstillseeplayer_ (message `/Game/States/AI_Sentry/DEV/I_AlertManagerDEV.SendStatus` _array_element))
    (`KismetArrayLibrary.Array_Add` (`self.CanSentrysSeePlayer?`) _canstillseeplayer_))
  (if (`KismetArrayLibrary.Array_Contains` (`self.CanSentrysSeePlayer?`) true)
    (`KismetArrayLibrary.Array_Clear` (`self.CanSentrysSeePlayer?`))
    (`KismetSystemLibrary.K2_SetTimerDelegate` (delegate `Check status of sentrys`) 1.0)
    (`KismetSystemLibrary.PrintString` "Still Hear" true true (struct :`G` 0.66 :`B` 1.0 :`A` 1.0) 0.5)
    (else
      (`KismetArrayLibrary.Array_Clear` (`self.CanSentrysSeePlayer?`))
      (`KismetSystemLibrary.PrintString` "All clear" true true (struct :`G` 0.66 :`B` 1.0 :`A` 1.0) 0.5))))

(event `AlertSystemON`)

(event `/Game/States/AI_Sentry/DEV/I_AlertManagerDEV.CheckStatus`)

(fn `SendStatus`
  (returns (`CanStillSeePLayer?` :type Boolean))
  (return false))

(fn `UserConstructionScript`)