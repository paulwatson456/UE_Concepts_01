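; Alert manager that tracks whether any AI sentry can still see the player after a guard spots them.
; PlayerSeenbyGuard starts a one-second timer that polls every I_AlertManager actor for sight status, re-arming while any reports true.
; When all report false it only prints "All clear".
; The activation broadcast and the timer to EnemyLost, which broadcasts deactivation, are unconnected, and SendStatus always returns false.
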(event `ContinueAlert`
  ;[1 0.01372 0.8946] Comment
  (`KismetSystemLibrary.K2_SetTimerDelegate` (delegate `Check status of sentrys`) 1.0))

(event `/Game/States/AI_Sentry/I_AlertManager.PlayerSeenByGuard`
  ;[1 0.01372 0.8946] Comment
  (`self.ContinueAlert`))

(event `Check status of sentrys`
  ;[1 0.01372 0.8946] Comment
  (bind _outactors (`GameplayStatics.GetAllActorsWithInterface` "/Game/States/AI_Sentry/I_AlertManager.I_AlertManager_C"))
  (for _array_element _outactors
    (bind _canstillseeplayer_ (message `/Game/States/AI_Sentry/I_AlertManager.SendStatus` _array_element))
    (`KismetArrayLibrary.Array_Add` (`self.CanSentrysSeePlayer?`) _canstillseeplayer_))
  (if (`KismetArrayLibrary.Array_Contains` (`self.CanSentrysSeePlayer?`) true)
    (`KismetArrayLibrary.Array_Clear` (`self.CanSentrysSeePlayer?`))
    (`self.ContinueAlert`)
    (`KismetSystemLibrary.PrintString` "Still Hear" true true (struct :`G` 0.66 :`B` 1.0 :`A` 1.0) 0.5)
    (else
      (`KismetArrayLibrary.Array_Clear` (`self.CanSentrysSeePlayer?`))
      (`KismetSystemLibrary.PrintString` "All clear" true true (struct :`G` 0.66 :`B` 1.0 :`A` 1.0) 0.5))))

(event `EnemyLost`
  ;[1 0.01372 0.8946] Comment
  (bind _outactors (`GameplayStatics.GetAllActorsWithInterface` "/Game/States/AI_Sentry/I_AlertManager.I_AlertManager_C"))
  (for _array_element _outactors
    (message `/Game/States/AI_Sentry/I_AlertManager.AlertSystemDeactivated` _array_element)))

(fn `SendStatus`
  (returns (`CanStillSeePLayer?` :type Boolean))
  (return false))

(fn `UserConstructionScript`)