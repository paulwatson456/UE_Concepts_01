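; BP_Door_Alert is a door that responds to the sentry alert system, closing when an alert activates and reopening when it ends.
; It starts open on BeginPlay, and the alert events call Open or Close, which slide DoorMesh vertically over a short timed move with MoveComponentTo.
; PlayerViewStatusCheck is a stub that always returns false.
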(event `self.ReceiveBeginPlay`
  (`self.Open`))

(event `/Game/States/AI_Sentry/I_AlertComms.AlertSystemActivated`
  ;[0 0.1061 1] DoorBP
  (`self.Close`))

(event `/Game/States/AI_Sentry/I_AlertComms.AlertSystemDeacivated`
  ;[0 0.1061 1] DoorBP
  (`self.Open`))

(event `Open`
  (`KismetSystemLibrary.MoveComponentTo` (`self.DoorMesh`) (0.0 0.0 340.0) (struct) false false 0.5))

(event `Close`
  (`KismetSystemLibrary.MoveComponentTo` (`self.DoorMesh`) (0.0 0.0 130.0) (struct) false false 0.5))

(fn `PlayerViewStatusCheck`
  (returns (`CanAISentrySeePlayer?` :type Boolean))
  (return false))

(fn `UserConstructionScript`)