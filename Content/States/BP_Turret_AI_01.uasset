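; Turret AI actor that sweeps a cube through a looping list of rotations until something overlaps its vision cone.
; A timeline lerps between rotation points, restarting from the first point when the overlap ends.
; During overlap, which is not filtered to the player, Tick turns the cube's yaw toward the player pawn at constant speed.
; A dot-product check prints a debug message once it nearly faces the player.
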(event `self.ReceiveBeginPlay`
  (`self.Move`))

(event `Move`
  (bind (_direction _newtrack_0) (`Timeline|Rotation` :!via `PlayFromStart` :!label _label)
    (:`Update`
      (`SceneComponent.K2_SetRelativeRotation` (`self.Cube`) (`KismetMathLibrary.RLerp` (`self.CurrentROT`) (`|GetArrayItem` (`self.RotationPoints`) (`self.PositionSelection`)) _newtrack_0) false false))
    (:`Finished`
      (bind _output_get (set `self.PositionSelection` (+ (`self.PositionSelection`) 1)))
      (if (>= _output_get (`KismetArrayLibrary.Array_Length` (`self.RotationPoints`)))
        (set `self.PositionSelection` 0)
        (set `self.CurrentROT` (`SceneComponent.RelativeRotation` (`self.Cube`)))
        (`self.Move`)
        (else
          (set `self.CurrentROT` (`SceneComponent.RelativeRotation` (`self.Cube`)))
          (`self.Move`))))))

(event `StopMove`
  (goto _label :!via `Stop`))

(event `self.VisionCone.OnComponentBeginOverlap`
  (params (OverlappedComponent :type "PrimitiveComponent Object Reference") (OtherActor :type "Actor Object Reference") (OtherComp :type "PrimitiveComponent Object Reference") (OtherBodyIndex :type Integer) (bFromSweep :type Boolean) (SweepResult :type "HitResult Structure (by ref)"))
  (set `self.PlayerSeen?` true)
  (`self.StopMove`))

(event `self.VisionCone.OnComponentEndOverlap`
  (params (OverlappedComponent :type "PrimitiveComponent Object Reference") (OtherActor :type "Actor Object Reference") (OtherComp :type "PrimitiveComponent Object Reference") (OtherBodyIndex :type Integer))
  (set `self.PlayerSeen?` false)
  (set `self.CurrentROT` (`SceneComponent.RelativeRotation` (`self.Cube`)))
  (set `self.PositionSelection` 0)
  (`self.Move`))

(event `self.ReceiveTick`
  (params (DeltaSeconds :type "Float (single-precision)"))
  (bind _cube (`self.Cube`))
  (bind (_returnvalue_roll _returnvalue_pitch _returnvalue_yaw) (`KismetMathLibrary.BreakRotator` (`KismetMathLibrary.RInterpTo_Constant` (`SceneComponent.K2_GetComponentRotation` (`self.Cube`)) (`KismetMathLibrary.FindLookAtRotation` (`SceneComponent.K2_GetComponentLocation` (`self.Cube`)) (`self.K2_GetActorLocation` (`GameplayStatics.GetPlayerPawn` 0))) DeltaSeconds 70.0)))
  (if (`self.PlayerSeen?`)
    (`SceneComponent.K2_SetRelativeRotation` (`self.Cube`) (`KismetMathLibrary.MakeRotator` 0.0 0.0 _returnvalue_yaw) false false)
    (if (> (`KismetMathLibrary.Dot_VectorVector` (`KismetMathLibrary.GetDirectionUnitVector` (`SceneComponent.K2_GetComponentLocation` _cube) (`self.K2_GetActorLocation` (`GameplayStatics.GetPlayerPawn` 0))) (`SceneComponent.GetForwardVector` _cube)) 0.98)
      (`KismetSystemLibrary.PrintString` "gotvcha"))))

(fn `UserConstructionScript`)