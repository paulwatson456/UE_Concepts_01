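; BP_Description is an interactable that shows a multi-line description or dialogue, one line per interaction.
; BeginPlay caches the text block from its WBP_DescriptionText widget component and hides the widget.
; Each Interact changes the BP_CC_States player state, reveals the widget and steps through the Dialogue array.
; The interaction after the last line resets the index, hides the widget and switches the player state back.
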(event `self.ReceiveBeginPlay`
  (set `self.MaxLineIndex` (`KismetArrayLibrary.Array_Length` (`self.Dialogue`)))
  (bind _aswbp_description_text (cast `/Game/States/WBP_DescriptionText` (`WidgetComponent.GetUserWidgetObject` (`self.W_description`))))
  (bind _output_get (set `self.As WBP Description Text` _aswbp_description_text))
  (set `self.Description Text` (`/Game/States/WBP_DescriptionText.DescriptionText` _output_get))
  (`Widget.SetVisibility` (`self.As WBP Description Text`) "Hidden"))

(event `/Game/States/I_GenInteract.Interact`
  (params (Inventory :type "Array of String (by ref)"))
  (bind _asbp_cc_states (cast `/Game/States/BP_CC_States` (`GameplayStatics.GetPlayerPawn` 0)))
  (set `/Game/States/BP_CC_States.StateOFPLayer` "NewEnumerator1" _asbp_cc_states)
  (`Widget.SetVisibility` (`self.As WBP Description Text`) "Visible")
  (`TextBlock.SetText` (`self.Description Text`) (`KismetTextLibrary.Conv_StringToText` (`|GetArrayItem` (`self.Dialogue`) (`self.CurrentLineIndex`))))
  (`/Engine/EditorBlueprintResources/StandardMacros.IncrementInt` (`self.CurrentLineIndex`)
    (:`  `
      (if (> (`self.CurrentLineIndex`) (`self.MaxLineIndex`))
        (set `self.CurrentLineIndex` 0)
        (`Widget.SetVisibility` (`self.As WBP Description Text`) "Hidden")
        (bind _asbp_cc_states_2 (cast `/Game/States/BP_CC_States` (`GameplayStatics.GetPlayerPawn` 0)))
        (set `/Game/States/BP_CC_States.StateOFPLayer` "NewEnumerator0" _asbp_cc_states_2)))))

(fn `UserConstructionScript`)