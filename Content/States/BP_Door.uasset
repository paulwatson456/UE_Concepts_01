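; BP_Door is a lockable, interactable door that requires a specific key from the interactor's inventory.
; It starts Locked, and Interact switches it to Unlocked if the inventory contains KeyRequired, otherwise printing the needed key while it stays locked.
; Once unlocked, each interaction toggles a FlipFlop that uses MoveComponentTo to swing DoorPivot open or closed around its yaw axis at its starting location.
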(event `self.ReceiveBeginPlay`
  (set `self.DoorState` "NewEnumerator0")
  (set `self.StartingLocation` (`SceneComponent.RelativeLocation` (`self.DoorPivot`))))

(event `/Game/States/I_GenInteract.Interact`
  (params (Inventory :type "Array of String (by ref)"))
  (if (`KismetArrayLibrary.Array_Contains` Inventory (`self.KeyRequired`))
    (set `self.DoorState` "NewEnumerator1"))
  (switch `/Game/States/E_OpenClose` (`self.DoorState`)
    (:`NewEnumerator0`
      (`KismetSystemLibrary.PrintString` (`KismetStringLibrary.Concat_StrStr` "Door loacked, you need the " (`self.KeyRequired`))))
    (:`NewEnumerator1`
      (`self.Open/Close`))))

(event `Open/Close`
  (`/Engine/EditorBlueprintResources/StandardMacros.FlipFlop`
    (:`A`
      (`KismetSystemLibrary.MoveComponentTo` (`self.DoorPivot`) (`self.StartingLocation`) (struct :`Yaw` 90.0) false false 1.0))
    (:`B`
      (`KismetSystemLibrary.MoveComponentTo` (`self.DoorPivot`) (`self.StartingLocation`) (struct) false false 1.0))))

(fn `UserConstructionScript`)